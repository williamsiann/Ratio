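; BP_Pila is a battery pickup actor that grants energy to whatever overlaps it.
; On box overlap it plays the Pila sound, sends a fixed energy amount to the overlapping actor through the ObtenerEnergia interface message, then destroys itself.
; A separate SumarEnergia function sets the character's hunger bar from its meter plus added energy, but the overlap does not call it.
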(event OnComponentBeginOverlap(Box)
  (params (OverlappedComponent :type Primitive%20Component%20Object%20Reference) (OtherActor :type Actor%20Object%20Reference) (OtherComp :type Primitive%20Component%20Object%20Reference) (OtherBodyIndex :type Integer) (bFromSweep :type Boolean) (SweepResult :type Hit%20Result%20Structure%20%28by%20ref%29))
  (Audio|PlaySound2D "/Game/Ratio/GAme/SoundMaster/Sound/Pila.Pila" 0.01 1.0 0.0 0 0)
  (Class|BPIRecolectar|ObtenerEnergia(Message) OtherActor 1e+01)
  (Actor|DestroyActor))

(fn ConstructionScript)

(fn SumarEnergia
  (bind _ref_ratio_char (Variables|Default|GetRef%20Ratio%20Char))
  (Progress|SetPercent (Variables|/Game/Ratio/Character/UserInterface/WB_Hambre.WB_Hambre_C|GetHambreBarra (Variables|/Game/Ratio/Character/BPZD_CharacterRatio.BPZD_CharacterRatio_C|GetStats%20ref (Variables|Default|GetRef%20Ratio%20Char))) (+ (Variables|/Game/Ratio/Character/BPZD_CharacterRatio.BPZD_CharacterRatio_C|GetMedidorHambre _ref_ratio_char) (Variables|/Game/Ratio/Character/BPZD_CharacterRatio.BPZD_CharacterRatio_C|GetSumEnergia _ref_ratio_char))))